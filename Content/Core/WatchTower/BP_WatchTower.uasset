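; BP_WatchTower is an input-driven camera rig that controls viewing distance and toggles a play mode.
; Mouse wheel steps the CameraBoom arm length in or out without clamping, while right mouse and Space snap it to near and very far presets.
; Escape flips IsPlayMode, calls OnPlayModeChanged, and hides the mouse cursor in play mode or shows it otherwise, with debug prints.
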(event `Key|MouseScrollUp`
  (params (Key :type "Key Structure"))
  (bind _cameraboom (`self.CameraBoom`))
  (:`Pressed`
    (set `SpringArmComponent.TargetArmLength` (+ (`SpringArmComponent.TargetArmLength` _cameraboom) 1000.0) _cameraboom)))

(event `Key|MouseScrollDown`
  (params (Key :type "Key Structure"))
  (bind _cameraboom (`self.CameraBoom`))
  (:`Pressed`
    (set `SpringArmComponent.TargetArmLength` (- (`SpringArmComponent.TargetArmLength` _cameraboom) 1000.0) _cameraboom)))

(event `Key|RightMouseButton`
  (params (Key :type "Key Structure"))
  (:`Pressed`
    (set `SpringArmComponent.TargetArmLength` 5000.0 (`self.CameraBoom`))
    (`KismetSystemLibrary.PrintString` "LOG_DEBUG: Set standard arm length: 5000")))

(event `Key|SpaceBar`
  (params (Key :type "Key Structure"))
  (:`Pressed`
    (set `SpringArmComponent.TargetArmLength` 200000.0 (`self.CameraBoom`))
    (`KismetSystemLibrary.PrintString` "LOG_DEBUG: Set standard arm length: 200000")))

(event `self.ReceiveBeginPlay`)

(event `Key|Escape`
  (params (Key :type "Key Structure"))
  (bind _returnvalue (`GameplayStatics.GetPlayerController` 0))
  (bind _isplaymode (`self.IsPlayMode`))
  (:`Pressed`
    (set `self.IsPlayMode` (not _isplaymode))
    (`self.OnPlayModeChanged`)
    (if _isplaymode
      (set `PlayerController.bShowMouseCursor` false _returnvalue)
      (`KismetSystemLibrary.PrintString` "OFF MOUSE CURSOR")
      (else
        (set `PlayerController.bShowMouseCursor` true _returnvalue)
        (`KismetSystemLibrary.PrintString` "SHOW MOUSE CURSOR")))))

(fn `UserConstructionScript`)